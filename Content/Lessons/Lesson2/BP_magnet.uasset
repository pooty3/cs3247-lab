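; BP_magnet is a lesson magnet actor that pulls actors inside its Box component toward its Target component.
; Every Tick it loops over the Box's overlapping actors, skipping itself, and offsets each by the unit direction to Target's world location.
; The pull is a one-unit step per frame without sweep, physics forces or delta-time scaling, so its speed depends on frame rate.
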(event `self.ReceiveTick`
  (params (DeltaSeconds :type "Float (single-precision)"))
  (for _array_element (`PrimitiveComponent.GetOverlappingActors` (`self.Box`) null)
    (if (not (== _array_element self))
      (`self.K2_AddActorWorldOffset` _array_element (`KismetMathLibrary.GetDirectionUnitVector` (`self.K2_GetActorLocation` _array_element) (`SceneComponent.K2_GetComponentLocation` (`self.target`))) false false))))

(fn `UserConstructionScript`)