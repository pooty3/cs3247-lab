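; BP_cannon is a cannon actor that repeatedly fires BP_flyingrock actors toward the world origin.
; The construction script rotates the root to face the origin, and a looping timer started on BeginPlay spawns rocks at the Cannonhead transform.
; Each rock receives a random velocity within a cone aimed at the origin and a rotation speed whose random ranges collapse to a constant.
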(event `self.ReceiveBeginPlay`
  (`KismetSystemLibrary.K2_SetTimerDelegate` (delegate `CustomEvent_0`) 2.0 true)
  (`KismetSystemLibrary.K2_SetTimer` null))

(event `CustomEvent_0`
  (bind _returnvalue (`KismetMathLibrary.RandomFloatInRange` 10.0 10.0))
  (bind _returnvalue_2 (`SceneComponent.K2_GetComponentToWorld` (`self.cannonhead`)))
  (bind _returnvalue_3 (`|SpawnActorFromClass` "/Game/Lessons/Lesson2/miniProject2/BP_flyingrock.BP_flyingrock_C" _returnvalue_2 "Undefined" "OverrideRootScale" null null))
  (set `/Game/Lessons/Lesson2/miniProject2/BP_flyingrock.movement` (* (`KismetMathLibrary.RandomUnitVectorInConeInDegrees` (`KismetMathLibrary.GetDirectionUnitVector` (`KismetMathLibrary.TransformLocation` _returnvalue_2)) 15.0) (`KismetMathLibrary.RandomFloatInRange` 1000.0 2000.0)) _returnvalue_3)
  (set `/Game/Lessons/Lesson2/miniProject2/BP_flyingrock.rotationspeed` (`KismetMathLibrary.MakeRotator` _returnvalue _returnvalue _returnvalue) _returnvalue_3))

(event `self.ReceiveTick`
  (params (DeltaSeconds :type "Float (single-precision)")))

(fn `UserConstructionScript`
  (`SceneComponent.K2_SetWorldRotation` (`self.DefaultSceneRoot`) (`KismetMathLibrary.FindLookAtRotation` (`SceneComponent.K2_GetComponentLocation` (`self.DefaultSceneRoot`)) (`KismetMathLibrary.MakeVector` 0.0)) false false))