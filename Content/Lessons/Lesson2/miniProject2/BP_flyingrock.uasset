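; A flying rock actor that moves and spins each tick, then explodes when it reaches the ground.
; Its construction script randomizes per-axis scale and picks one of three meshes: capsule, cannonball or cone.
; Tick applies the Rotationspeed and Movement variables scaled by delta time, without sweeping.
; Overlapping an actor tagged "ground" spawns an asteroid explosion effect and sound, then destroys the rock.
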(event `self.ReceiveTick`
  (params (DeltaSeconds :type "Float (single-precision)"))
  (`self.K2_AddActorLocalRotation` (* (`self.rotationspeed`) DeltaSeconds))
  (`self.K2_AddActorWorldOffset` (* (`self.movement`) DeltaSeconds)))

(event `self.StaticMesh.OnComponentBeginOverlap`
  (params (OverlappedComponent :type "PrimitiveComponent Object Reference") (OtherActor :type "Actor Object Reference") (OtherComp :type "PrimitiveComponent Object Reference") (OtherBodyIndex :type Integer) (bFromSweep :type Boolean) (SweepResult :type "HitResult Structure (by ref)"))
  (bind _returnvalue (`self.K2_GetActorLocation`))
  (if (`self.ActorHasTag` OtherActor "ground")
    (`GameplayStatics.SpawnEmitterAtLocation` "/Game/Effects/Particles/Explosion/P_AsteroidExplosion.P_AsteroidExplosion" _returnvalue)
    (`GameplayStatics.PlaySoundAtLocation` "/Game/Audio/SoundWaves/Effect/SW_Explosion_1.SW_Explosion_1" _returnvalue (struct) 0.1 1.0 0.0 null null null)
    (`self.K2_DestroyActor`)))

(fn `NewFunction_0`
  (bind _returnvalue (`KismetMathLibrary.RandomFloatInRange` 0.8 2.0))
  (bind _staticmesh (`self.StaticMesh`))
  (`SceneComponent.SetWorldScale3D` (`self.DefaultSceneRoot`) (`KismetMathLibrary.MakeVector` _returnvalue _returnvalue _returnvalue))
  (switch `int` (`KismetMathLibrary.RandomIntegerInRange` 0 2)
    (:`Default`
      (`StaticMeshComponent.SetStaticMesh` _staticmesh "/Game/Meshes/Architecture/BuildingBlocks/Shapes/Shape_Cone.Shape_Cone"))
    (:`0`
      (`StaticMeshComponent.SetStaticMesh` _staticmesh "/Game/Meshes/Architecture/BuildingBlocks/Shapes/Shape_Capsule_A.Shape_Capsule_A"))
    (:`1`
      (`StaticMeshComponent.SetStaticMesh` _staticmesh "/Game/Meshes/Props/Combat/Ammo/SM_Cannonball.SM_Cannonball"))))

(fn `UserConstructionScript`
  (`self.NewFunction_0`))